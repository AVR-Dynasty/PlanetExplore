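; BP_Resource is a world resource actor whose appearance comes from a data asset and which shows a hint when the player is near.
; The construction script sets ResourceMesh from the mesh in ResourceDataAsset when that asset is valid.
; HintBox overlap events show HintWidget when a BP_ThirdPersonCharacter enters and hide it on exit.
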(event `self.HintBox.OnComponentBeginOverlap`
  (params (OverlappedComponent :type "PrimitiveComponent Object Reference") (OtherActor :type "Actor Object Reference") (OtherComp :type "PrimitiveComponent Object Reference") (OtherBodyIndex :type Integer) (bFromSweep :type Boolean) (SweepResult :type "HitResult Structure (by ref)"))
  (cast `/Game/ThirdPerson/Blueprints/BP_ThirdPersonCharacter` OtherActor)
  (`SceneComponent.SetVisibility` (`self.HintWidget`) true false))

(event `self.HintBox.OnComponentEndOverlap`
  (params (OverlappedComponent :type "PrimitiveComponent Object Reference") (OtherActor :type "Actor Object Reference") (OtherComp :type "PrimitiveComponent Object Reference") (OtherBodyIndex :type Integer))
  (cast `/Game/ThirdPerson/Blueprints/BP_ThirdPersonCharacter` OtherActor)
  (`SceneComponent.SetVisibility` (`self.HintWidget`) false false))

(fn `UserConstructionScript`
  (bind _resourcedataasset (`self.ResourceDataAsset`))
  (`/Engine/EditorBlueprintResources/StandardMacros.IsValid` _resourcedataasset
    (:`Is Valid`
      (`StaticMeshComponent.SetStaticMesh` (`self.ResourceMesh`) (`/Game/DataAsset/ResourceData/PDA_ResourceData.Mesh` _resourcedataasset)))))